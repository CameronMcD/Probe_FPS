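; Key-locked door Blueprint that opens when a FirstPersonCharacter carrying enough keys enters its overlap volume.
; On overlap it deducts RequiredNumberOfKeys from the character and plays the DoorMovement timeline, lerping the Door's relative location from the origin to TargetLocation.
; Any actor leaving the volume reverses the timeline after a two-second delay, closing the door.
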(event OnComponentBeginOverlap(Overlap)
  (params (OverlappedComponent :type Primitive%20Component%20Object%20Reference) (OtherActor :type Actor%20Object%20Reference) (OtherComp :type Primitive%20Component%20Object%20Reference) (OtherBodyIndex :type Integer) (bFromSweep :type Boolean) (SweepResult :type Hit%20Result%20Structure%20%28by%20ref%29))
  (bind _requirednumberofkeys (Variables|Default|GetRequiredNumberOfKeys))
  ;[1 1 1] Door mechanic, checks the current number of keys is >= current keys, if true keys are removed and door animation is played.
  (bind _asfirst_person_character (Utilities|Casting|CastToFirstPersonCharacter OtherActor))
  (if (>= (Variables|/Game/FirstPersonBP/Blueprints/FirstPersonCharacter.FirstPersonCharacter_C|GetNumberOfKeys _asfirst_person_character) _requirednumberofkeys)
    (Variables|/Game/FirstPersonBP/Blueprints/FirstPersonCharacter.FirstPersonCharacter_C|SetNumberOfKeys _asfirst_person_character (- (Variables|/Game/FirstPersonBP/Blueprints/FirstPersonCharacter.FirstPersonCharacter_C|GetNumberOfKeys _asfirst_person_character) _requirednumberofkeys))
    (bind _alpha (Timeline|DoorMovement Play)
      (:Update
        (Transformation|SetRelativeLocation (Variables|Default|GetDoor) (Math|Vector|Lerp(Vector) "0, 0, 0" (Variables|Default|GetTargetLocation) _alpha) false false)))))

(event OnComponentEndOverlap(Overlap)
  (params (OverlappedComponent :type Primitive%20Component%20Object%20Reference) (OtherActor :type Actor%20Object%20Reference) (OtherComp :type Primitive%20Component%20Object%20Reference) (OtherBodyIndex :type Integer))
  ;[1 1 1] Door mechanic, checks the current number of keys is >= current keys, if true keys are removed and door animation is played.
  (Utilities|FlowControl|Delay 2.0)
  (bind _alpha (Timeline|DoorMovement Reverse)
    (:Update
      (Transformation|SetRelativeLocation (Variables|Default|GetDoor) (Math|Vector|Lerp(Vector) "0, 0, 0" (Variables|Default|GetTargetLocation) _alpha) false false))))

(fn ConstructionScript)